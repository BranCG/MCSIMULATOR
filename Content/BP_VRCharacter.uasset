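; BP_VRCharacter is a VR character that records speech while the trigger-recording input is held and sends it for analysis.
; SpeechRecorder starts and stops with the input action, then passes raw PCM data to SpeechAnalyzer on stop.
; Completed results go to a BP_VRFeedbackActor found by class lookup for display, while failures print their error message.
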(event `EnhancedInput|/Game/IA_TriggerRecording`
  (params (ActionValue :type Boolean) (ElapsedSeconds :type "Float (double-precision)") (TriggeredSeconds :type "Float (double-precision)") (InputAction :type "InputAction Object Reference" :default "/Game/IA_TriggerRecording.IA_TriggerRecording"))
  (:`Started`
    (`SpeechRecorderComponent.StartRecording` (`self.SpeechRecorder`)))
  (:`Completed`
    (`SpeechRecorderComponent.StopRecording` (`self.SpeechRecorder`))))

(event `self.SpeechRecorder.OnRecordingStopped`
  (params (RawPCMData :type "Array of Byte (by ref)"))
  (`SpeechAnalyzer.RequestSpeechAnalysis` (`self.SpeechAnalyzer`) RawPCMData))

(event `self.SpeechAnalyzer.OnAnalysisCompleted`
  (params (Result :type "SpeechAnalysisResult Structure (by ref)"))
  (bind _returnvalue (`GameplayStatics.GetActorOfClass` "/Game/BP_VRFeedbackActor.BP_VRFeedbackActor_C"))
  (`VRFeedbackActor.DisplayAnalysisResults` _returnvalue Result))

(event `self.SpeechAnalyzer.OnAnalysisFailed`
  (params (ErrorMessage :type String))
  (`KismetSystemLibrary.PrintString` ErrorMessage))

(fn `UserConstructionScript`)